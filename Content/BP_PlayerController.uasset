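; Player controller that provides keyboard controls for the BP_Cloth actor in the level.
; R resets the cloth and P releases it.
; Holding L sets a painting flag, and Tick then adds a random burn to the cloth every frame while it is set.
; Each action looks up the cloth with GetActorOfClass at the moment it runs.
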(event EventBeginPlay)

(event EventTick
  (params (DeltaSeconds :type Float%20%28single-precision%29))
  (if (Variables|Default|GetPaintingCloth)
    (bind _returnvalue (Actor|GetActorOfClass "/Game/BP_Cloth.BP_Cloth_C"))
    (Class|Cloth|AddRandomBurn _returnvalue)))

(event Input|KeyboardEvents|L
  (params (Key :type Key%20Structure :default "None"))
  (:Pressed
    (Variables|Default|SetPaintingCloth true))
  (:Released
    (Variables|Default|SetPaintingCloth false)))

(event Input|KeyboardEvents|R
  (params (Key :type Key%20Structure :default "None"))
  (:Pressed
    (bind _returnvalue (Actor|GetActorOfClass "/Game/BP_Cloth.BP_Cloth_C"))
    (Utilities|IsValid _returnvalue
      (:Is%20Valid
        (Class|Cloth|ResetCloth _returnvalue)))))

(event Input|KeyboardEvents|P
  (params (Key :type Key%20Structure :default "None"))
  (:Pressed
    (bind _returnvalue (Actor|GetActorOfClass "/Game/BP_Cloth.BP_Cloth_C"))
    (Utilities|IsValid _returnvalue
      (:Is%20Valid
        (Class|Cloth|ReleaseCloth _returnvalue)))))

(fn ConstructionScript)