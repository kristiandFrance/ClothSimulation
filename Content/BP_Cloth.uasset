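; BP_Cloth is an actor that displays wind with an arrow, judging by its variables and components.
; Each tick it sets the ArrowRoot world rotation to WindRotation.
; It also stretches the Arrow along X by lerping between fixed bounds, using total wind strength offset by the minimum, divided by the maximum and multiplied by local wind strength.
; The file shows no cloth simulation logic and an empty construction script.
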(event Collision|EventActorBeginOverlap
  (params (OtherActor :type Actor%20Object%20Reference)))

(event EventTick
  (params (DeltaSeconds :type Float%20%28single-precision%29))
  (Transformation|SetWorldRotation (Variables|Default|GetArrowRoot) (Variables|Default|GetWindRotation) false false)
  (Transformation|SetWorldScale3D (Variables|Default|GetArrow) (Math|Vector|MakeVector (Math|Float|Lerp 1.0 5.0 (* (/ (- (Variables|Default|GetTotalWindStrength) (Variables|Default|GetMinWindStrength)) (Variables|Default|GetMaxWindStrength)) (Variables|Default|GetLocalWindStrength))) 2.0 2.0)))

(fn ConstructionScript)